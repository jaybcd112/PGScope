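; Ladder zone Blueprint that builds a climbable ladder of adjustable height and keeps positions within it.
; The construction script sorts the endpoints into a vertical span, sizes the box volume, generates transitions and stacks instanced step meshes with a flipped exit step.
; With step constraint on, position queries snap local height to every second step before parent clamping, and directional queries ignore the desired delta.
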(fn ConstructionScript
  (Utilities|FlowControl|Sequence
    (:then_0
      ;[0.1 0.1 0.1] Sort ladder variables
      (LocalVariables|SetTemp%20Start (Math|Vector|MakeVector (.X (Math|Vector|BreakVector (Variables|Default|GetZoneStart))) (.Y (Math|Vector|BreakVector (Variables|Default|GetZoneStart))) (Math|Float|Min(Float) (.Z (Math|Vector|BreakVector (Variables|Default|GetZoneStart))) (.Z (Math|Vector|BreakVector (Variables|Default|GetZoneEnd))))))
      (Variables|Default|SetZoneEnd (Math|Vector|MakeVector (.X (Math|Vector|BreakVector (Variables|Default|GetZoneStart))) (.Y (Math|Vector|BreakVector (Variables|Default|GetZoneStart))) (Math|Float|Max(Float) (.Z (Math|Vector|BreakVector (Variables|Default|GetZoneStart))) (.Z (Math|Vector|BreakVector (Variables|Default|GetZoneEnd))))))
      (Variables|Default|SetZoneStart (LocalVariables|GetTemp%20Start))
      (LocalVariables|SetHeight (.Z (Math|Vector|BreakVector (Variables|Default|GetZoneEnd))))
      (Variables|Ladder|SetOverlap%20Depth (/ (+ (.x (Variables|Ladder|GetOverlap%20Extent)) (Variables|Ladder|GetDepth)) 2.0)))
    (:then_1
      ;[0.1 0.1 0.1] Position Box Volume
      (Components|Box|SetBoxExtent (Variables|Default|GetExtend) (Math|Vector|MakeVector (Variables|Ladder|GetOverlap%20Depth) (Variables|Ladder|GetWidth) (* (LocalVariables|GetHeight) 0.5)) true)
      (Transformation|SetRelativeLocation (Variables|Default|GetExtend) (Math|Vector|MakeVector (- (Variables|Ladder|GetOverlap%20Depth) (Variables|Ladder|GetDepth)) 0.0 (* (LocalVariables|GetHeight) 0.5)) false false))
    (:then_2
      ;[0.1 0.1 0.1] Create Meshes
      (Utilities|FlowControl|Sequence
        (:then_0
          ;;[0.1 0.1 0.1] Calculate how many steps are needed
          (Variables|Ladder|SetStep%20Count (Math|Float|Floor (/ (LocalVariables|GetHeight) (Variables|Ladder|GetStep%20Height))))
          ;;[0.1 0.1 0.1] Create Transitions
          (Class|AdvKitZone|GenerateTransitions true))
        (:then_1
          ;;[0.1 0.1 0.1] Create ladder meshes
          (for _index (range 0 (- (Variables|Ladder|GetStep%20Count) 2))
            (Components|InstancedStaticMesh|AddInstance (Variables|Default|GetLadder%20Mesh) (Math|Transform|MakeTransform (Math|Vector|MakeVector 0.0 0.0 (* _index (Variables|Ladder|GetStep%20Height))) "0, 0, 0" "1.000000,1.000000,1.000000"))))
        (:then_2
          ;;[0.1 0.1 0.1] Add exit step
          (Components|InstancedStaticMesh|AddInstance (Variables|Default|GetLadder%20Mesh) (Math|Transform|MakeTransform (Math|Vector|MakeVector 0.0 0.0 (- (* (Variables|Ladder|GetStep%20Count) (Variables|Ladder|GetStep%20Height)) 3.0)) "0, 0,180.000000" "1.000000,1.000000,1.000000")))))))

(fn ConstrainPositiontoZone
  (params (WorldPosition :type Vector%20%28by%20ref%29 :default "0, 0, 0") (HalfExtent :type Vector%20%28by%20ref%29 :default "0, 0, 0") (ExtentWorldRotation :type Rotator%20%28by%20ref%29 :default "0, 0, 0"))
  (bind _self self)
  (bind _step_height (Variables|Ladder|GetStep%20Height))
  (bind _returnvalue (Transformation|GetActorTransform _self))
  (bind _returnvalue_2 (* _step_height 2.0))
  ;[0.1 0.1 0.1] Constrain given position to closest ladder step
  (if (Variables|Ladder|GetConstrain%20To%20Steps)
    (return (|CallParentFunction (Math|Transform|TransformLocation _returnvalue (Math|Vector|MakeVector 0.0 0.0 (* (Math|Float|Round (/ (.z (Math|Transform|InverseTransformLocation _returnvalue WorldPosition)) _returnvalue_2)) _returnvalue_2))) HalfExtent ExtentWorldRotation))
    (else
      (return (|CallParentFunction WorldPosition HalfExtent ExtentWorldRotation)))))

(fn GetPositioninDirection
  (params (FromWorldPosition :type Vector%20%28by%20ref%29 :default "0, 0, 0") (WorldDesiredDelta :type Vector%20%28by%20ref%29 :default "0, 0, 0") (bClamp :type Boolean) (HalfExtent :type Vector%20%28by%20ref%29 :default "0, 0, 0") (ExtentWorldRotation :type Rotator%20%28by%20ref%29 :default "0, 0, 0"))
  (if (Variables|Ladder|GetConstrain%20To%20Steps)
    (return (CallFunction|ConstrainPositiontoZone FromWorldPosition HalfExtent ExtentWorldRotation))
    (else
      (bind _returnvalue (|CallParentFunction FromWorldPosition WorldDesiredDelta bClamp HalfExtent ExtentWorldRotation))
      (return _returnvalue))))